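; BP_DTDragDropFile is an actor that logs files and folders dragged from the operating system onto the game window.
; On BeginPlay it shows the mouse cursor, adds a UI_LOG widget to the viewport and switches to a fixed-size windowed resolution through a console command.
; The DTSystemDragDropFile drop event supplies separate file and folder path lists, which it writes to that log under headings with a closing separator.
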(event `self.ReceiveBeginPlay`
  (set `PlayerController.bShowMouseCursor` true (`GameplayStatics.GetPlayerController` 0))
  (bind _returnvalue (`|CreateWidget` "/Game/UI_LOG.UI_LOG_C"))
  (bind _output_get (set `self.Log` _returnvalue))
  (`UserWidget.AddToViewport` _output_get 0)
  (`KismetSystemLibrary.ExecuteConsoleCommand` "r.setRes 1024 x 768w" null))

(event `self.DTSystemDragDropFile.OnSystemDragDropFile`
  (params (FilePathList :type "Array of String (by ref)") (FolderPathList :type "Array of String (by ref)"))
  (`/Game/UI_LOG.AddLog` (`self.Log`) "File : ")
  (for _array_element FilePathList
    (`/Game/UI_LOG.AddLog` (`self.Log`) _array_element))
  (`/Game/UI_LOG.AddLog` (`self.Log`) "Folder : ")
  (for _array_element_2 FolderPathList
    (`/Game/UI_LOG.AddLog` (`self.Log`) _array_element_2))
  (`/Game/UI_LOG.AddLog` (`self.Log`) "End -------------------------------------------------------"))

(fn `UserConstructionScript`)